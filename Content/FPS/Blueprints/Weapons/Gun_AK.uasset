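; AK gun Blueprint for the first-person pawn, overriding its parent's ammo, reload time and spread defaults.
; Fire spends ammo, traces from the camera with random spread, then spawns an impact decal, tracer and randomized muzzle flash, or dry-fires when empty.
; A second muzzle-to-impact trace runs but its result is unused, and no damage is applied here.
; Reload plays a montage, then refills ammo after a delay.
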(event EventFire
  (if (> (Variables|Default|GetAmmoCount) 0)
    (CallFunction|AmmoCheck)
    (bind (_muzzlelocation _impactpoint) (CallFunction|LineTrace))
    (CallFunction|SpawnDecalTracer _muzzlelocation _impactpoint _impactpoint)
    (Utilities|MuzzleFlash)
    (else
      (Audio|PlaySoundatLocation "/Game/FPS/Audio/DryFire.DryFire" (Transformation|GetWorldLocation (Variables|/Game/FPS/Blueprints/FPSPawn_BP.FPSPawn_BP_C|GetFirstPersonCamera (.AsFPSPawn%20BP (Utilities|Casting|CastToFPSPawn_BP (Game|GetPlayerCharacter 0))))) "0, 0, 0" 1.0 1.0 0.0 0 0 0))))

(event EventReload
  (Components|Animation|PlayAnimation (Variables|Default|GetPrimaryWeapon) "/Game/FPS/Animations/AK_Reload_anim_Anim_Montage.AK_Reload_anim_Anim_Montage" false)
  (Utilities|FlowControl|Delay (Variables|Default|GetReloadTime))
  (Variables|Default|SetAmmoCount (Variables|Default|GetMaxAmmo)))

(fn ConstructionScript
  (|CallParentFunction)
  (Variables|Default|SetMaxAmmo 30)
  (Variables|Default|SetAmmoCount 30)
  (Variables|Default|SetReloadTime 2.0)
  (Variables|Default|SetBulletSpread 5e+02))

(fn AmmoCheck
  (bind _returnvalue (Math|Random|RandomFloatinRange 0.7 1.2))
  (Math|Integer|DecrementInt (Variables|Default|GetAmmoCount)
    (:%20%20
      (if (not (Variables|/Game/FPS/Blueprints/FPSPawn_BP.FPSPawn_BP_C|GetIsReloading (.AsFPSPawn%20BP (Utilities|Casting|CastToFPSPawn_BP (Game|GetPlayerCharacter 0)))))
        (Audio|PlaySoundatLocation "/Game/FPS/Audio/Gunshot.Gunshot" (Transformation|GetWorldLocation (Variables|/Game/FPS/Blueprints/FPSPawn_BP.FPSPawn_BP_C|GetFirstPersonCamera (.AsFPSPawn%20BP (Utilities|Casting|CastToFPSPawn_BP (Game|GetPlayerCharacter 0))))) "0, 0, 0" (+ _returnvalue 2.5) _returnvalue 0.0 0 0 0)
        (Components|Animation|PlayAnimation (Variables|Default|GetPrimaryWeapon) "/Game/FPS/Animations/AK_Fire_anim_Anim.AK_Fire_anim_Anim" false)))))

(fn LineTrace
  (bind _returnvalue (Game|GetPlayerCharacter 0))
  (bind _bulletspread (Variables|Default|GetBulletSpread))
  (bind _muzzle (Variables|Default|GetMuzzle))
  (bind _returnvalue_2 (Transformation|GetWorldLocation _muzzle))
  (bind _returnvalue_3 (* _bulletspread -1.0))
  (bind _asfpspawn_bp (Utilities|Casting|CastToFPSPawn_BP _returnvalue))
  (bind _firstpersoncamera (Variables|/Game/FPS/Blueprints/FPSPawn_BP.FPSPawn_BP_C|GetFirstPersonCamera _asfpspawn_bp))
  (bind _returnvalue_4 (Transformation|GetWorldLocation _firstpersoncamera))
  (bind _outhit (Collision|LineTraceByChannel _returnvalue_4 (+ (+ (* (Math|Vector|GetForwardVector _firstpersoncamera) 2e+04) _returnvalue_4) (Math|Vector|MakeVector (Math|Random|RandomFloatinRange _returnvalue_3 _bulletspread) (Math|Random|RandomFloatinRange _returnvalue_3 _bulletspread) (Math|Random|RandomFloatinRange _returnvalue_3 _bulletspread))) "TraceTypeQuery1" false 0 "None")) ; CameraShot
  (Collision|LineTraceByChannel _returnvalue_2 (.ImpactPoint (Collision|BreakHitResult _outhit)) "TraceTypeQuery1" false 0 "None" true "(R=0.000000,G=1.000000,B=0.016391,A=1.000000)") ; GunShot
  (return _returnvalue_2 (.ImpactPoint (Collision|BreakHitResult _outhit))))

(fn SpawnDecalTracer
  (params (Location :type Vector) (SpawnTransformLocation :type Vector) (ImpactPoint :type Vector))
  (Game|SpawnActorfromClass "/Game/FPS/Blueprints/BulletDecal_BP.BulletDecal_BP_C" (Math|Transform|MakeTransform SpawnTransformLocation (Math|Conversions|RotationFromXVector ImpactPoint) "0.025000,0.025000,0.025000") "Undefined" 0 0)
  (if (>= (Math|Random|RandomIntegerinRange 1 10) 0)
    (Game|SpawnActorfromClass "/Game/FPS/Blueprints/TracerRounds_BP.TracerRounds_BP_C" (Math|Transform|MakeTransform Location (Transformation|GetWorldRotation (Variables|/Game/FPS/Blueprints/FPSPawn_BP.FPSPawn_BP_C|GetFirstPersonCamera (.AsFPSPawn%20BP (Utilities|Casting|CastToFPSPawn_BP (Game|GetPlayerCharacter 0))))) "0.050000,0.050000,0.050000") "Undefined" 0 0))
  (return))